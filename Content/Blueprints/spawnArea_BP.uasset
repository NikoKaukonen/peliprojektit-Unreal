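; spawnArea_BP is an asteroid spawner that sends Asteroid_BP actors toward the player's ship.
; After a startup delay, a looping timer at SpawnDelay spawns an asteroid and sets its MovementDirection toward the ship's collider.
; GetSpawnArea samples random SpawnVolume points, but tests the NegativeVolume extent only on zeroed coordinates before sampling.
; RandomizeSpawnDelay is never called, and debug prints remain throughout.
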(event Custom|CustomEvent_Randomize_Spawn_Delay
  (bind _spawn_coordinates (CallFunction|GetSpawnArea))
  (Development|PrintString (Utilities|String|ToString(Vector) _spawn_coordinates))
  (bind _returnvalue (Game|SpawnActorfromClass "/Game/Blueprints/asteroid_BP.asteroid_BP_C" (Math|Transform|MakeTransform _spawn_coordinates "0, 0, 0" "1.000000,1.000000,1.000000") "AdjustIfPossibleButDontSpawnIfColliding" "MultiplyWithRoot" 0 0))
  (bind _output_get (Variables|Default|Setspawned_asteroid _returnvalue))
  (bind _move_direction (CallFunction|GetDirection "0, 0, 0" _output_get))
  (Variables|/Game/Blueprints/asteroid_BP.asteroid_BP_C|SetmovementDirection _output_get _move_direction))

(event EventBeginPlay
  (Variables|Default|Setpositive_volume (Variables|Default|Getpositive_volume))
  (Variables|Default|Setnegative_volume (Variables|Default|Getnegative_volume))
  (Utilities|FlowControl|Delay 3.0)
  (Variables|Default|Setis_spawning? true)
  (Utilities|Time|SetTimerbyEvent (delegate Custom|CustomEvent_Randomize_Spawn_Delay) (Variables|Default|Getspawn_delay) true true 0.1))

(fn ConstructionScript)

(fn GetSpawnArea
  (bind _spawn_volume (Variables|Default|Getspawn_volume))
  (bind _returnvalue (Transformation|GetWorldLocation _spawn_volume))
  (bind _boxextent (Variables|/Script/Engine.BoxComponent|GetBoxExtent _spawn_volume))
  (bind _returnvalue_2 (Math|Random|RandomPointinBoundingBox _returnvalue _boxextent))
  (Variables|Default|SetSpawn%20Coordinates%20Z_TEMP 0.0)
  (Variables|Default|SetSpawn%20Coordinates%20Y_TEMP 0.0)
  (Variables|Default|SetSpawn%20Coordinates%20X_TEMP 0.0)
  (Development|PrintString "getting spawn area.")
  (if (Math|Geometry|IsPointinBox (Math|Vector|MakeVector (stale _output_get) (stale _output_get_2) (stale _output_get_3)) _returnvalue (Variables|/Script/Engine.BoxComponent|GetBoxExtent (Variables|Default|Getnegative_volume)))
    (Utilities|FlowControl|ForLoopwithBreak 0 (Variables|Default|Getretries) :!label _label
      (:LoopBody
        (bind _output_get (Variables|Default|SetSpawn%20Coordinates%20X_TEMP (.x _returnvalue_2)))
        (bind _output_get_2 (Variables|Default|SetSpawn%20Coordinates%20Y_TEMP (.y _returnvalue_2)))
        (bind _output_get_3 (Variables|Default|SetSpawn%20Coordinates%20Z_TEMP (.z _returnvalue_2))))
      (:Completed
        (Development|PrintString "Valid spawn found.")
        (bind _output_get_4 (Variables|Default|SetSpawn%20Coordinates%20X _output_get))
        (Development|PrintString (Utilities|String|ToString(Float) _output_get_4))
        (bind _output_get_5 (Variables|Default|SetSpawn%20Coordinates%20Y _output_get_2))
        (Development|PrintString (Utilities|String|ToString(Float) _output_get_5))
        (bind _output_get_6 (Variables|Default|SetSpawn%20Coordinates%20Z _output_get_3))
        (Development|PrintString (Utilities|String|ToString(Float) _output_get_6))
        (return (Math|Vector|MakeVector _output_get_4 _output_get_5 _output_get_6))))
    (else
      (goto _label Break))))

(fn RandomizeSpawnDelay
  (bind _output_get (Variables|Default|Setspawn_delay (Math|Random|RandomFloatinRange 1.0 5.0)))
  (Development|PrintString "Spawn delay: ")
  (Development|PrintString (Utilities|String|ToString(Float) _output_get))
  (return))

(fn GetDirection
  (params (asteroid_spawn_location :type Vector) (asteroid :type Actor%20Object%20Reference))
  (bind _asship__bp (Utilities|Casting|CastToship__BP (Game|Player|GetPlayerPawn 0)))
  (bind _asasteroid_bp (Utilities|Casting|CastToasteroid_BP asteroid))
  (bind _output_get (Variables|Default|Setdirection (- (Transformation|GetWorldLocation (Variables|/Game/Blueprints/ship__BP.ship__BP_C|Getship_collider _asship__bp)) (Transformation|GetWorldLocation (Variables|/Game/Blueprints/asteroid_BP.asteroid_BP_C|Getasteroid_collider _asasteroid_bp)))))
  (return (Math|Vector|Normalize _output_get)))