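; Player-controlled ship Blueprint with thrust, rotation and wrap-around movement within a rectangular play area.
; On BeginPlay it adds the Controls Enhanced Input mapping context for its player controller.
; Thrust applies a velocity-change impulse along the ShipCollider's forward vector, spin adds yaw directly, and the shoot input is an empty stub.
; Tick wraps the ship by negating X or Y whenever it leaves the fixed bounds.
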(event Input|EnhancedActionEvents|EnhancedInputActionthrustIA
  (params (ActionValue :type Vector%202D%20Structure) (ElapsedSeconds :type Float%20%28double-precision%29) (TriggeredSeconds :type Float%20%28double-precision%29) (InputAction :type Input%20Action%20Object%20Reference :default "/Game/Blueprints/thrustIA.thrustIA"))
  (Physics|AddImpulse (Variables|Default|Getship_collider) (* (Math|Vector|GetForwardVector (Transformation|GetWorldRotation (Variables|Default|Getship_collider))) (Variables|Default|GetshipSpeed)) "None" true))

(event Input|EnhancedActionEvents|EnhancedInputActionshootIA
  (params (ActionValue :type Boolean) (ElapsedSeconds :type Float%20%28double-precision%29) (TriggeredSeconds :type Float%20%28double-precision%29) (InputAction :type Input%20Action%20Object%20Reference :default "/Game/Blueprints/shootIA.shootIA")))

(event Input|EnhancedActionEvents|EnhancedInputActionspinAI
  (params (ActionValue :type Vector%202D%20Structure) (ElapsedSeconds :type Float%20%28double-precision%29) (TriggeredSeconds :type Float%20%28double-precision%29) (InputAction :type Input%20Action%20Object%20Reference :default "/Game/Blueprints/spinAI.spinAI"))
  (Transformation|AddRelativeRotation (Variables|Default|Getship_collider) (Math|Rotator|MakeRotator 0.0 0.0 (+ (.x ActionValue) (.y ActionValue))) false false))

(event EventBeginPlay
  (bind _asplayer_controller (Utilities|Casting|CastToPlayerController (Pawn|GetController)))
  (Utilities|IsValid (PlayerController|LocalPlayerSubsystems|GetEnhancedInputLocalPlayerSubsystem _asplayer_controller)
    (:Is%20Valid
      (Input|AddMappingContext (PlayerController|LocalPlayerSubsystems|GetEnhancedInputLocalPlayerSubsystem _asplayer_controller) "/Game/Blueprints/controls.controls" 0 "(bIgnoreAllPressedKeysUntilRelease=True,bForceImmediately=False,bNotifyUserSettings=False)"))))

(event EventTick
  (params (DeltaSeconds :type Float%20%28single-precision%29))
  (bind _returnvalue (Transformation|GetActorLocation))
  (bind _returnvalue_2 (Transformation|GetActorLocation))
  (bind (_x _y _z) (Math|Vector|BreakVector _returnvalue))
  (bind (_x_2 _y_2 _z_2) (Math|Vector|BreakVector _returnvalue_2))
  (if (not (Math|Float|InRange(Float) _y_2 -1.1e+03 1.1e+03))
    (Transformation|SetActorLocation (Math|Vector|MakeVector _x_2 (* _y_2 -1.0) _z_2) false false))
  (if (not (Math|Float|InRange(Float) _x -1.4e+03 1.4e+03))
    (Transformation|SetActorLocation (Math|Vector|MakeVector (* _x -1.0) _y _z) false false)))

(fn ConstructionScript)