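; Planet actor that drifts through the world while spinning, with randomized size and speed.
; BeginPlay picks a random scale for each axis independently and a random movement speed.
; Tick offsets the root along MovementDirection and adds a small random yaw, both per frame without delta-time scaling.
; Disconnected leftover nodes hold an alternate randomization, a ship lookup and lifetime-based destruction, none of which runs.
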(event EventBeginPlay
  (bind _returnvalue (Math|Random|RandomFloatinRange 3.0 2e+01))
  ;[1 1 1] Randomize base values.
  (Transformation|SetRelativeScale3D (Variables|Default|GetDefaultSceneRoot) (Math|Vector|MakeVector _returnvalue _returnvalue _returnvalue))
  (Variables|Default|SetMovement%20Speed (Math|Random|RandomFloatinRange 1.0 1e+01)))

(event EventTick
  (params (DeltaSeconds :type Float%20%28single-precision%29))
  ;[1 1 1] Update rotation and location once per frame.
  (Transformation|AddWorldOffset (Variables|Default|GetDefaultSceneRoot) (* (Variables|Default|GetmovementDirection) (Variables|Default|GetMovement%20Speed)) false false)
  (Transformation|AddLocalRotation (Variables|Default|GetDefaultSceneRoot) (Math|Rotator|MakeRotator 0.0 0.0 (Math|Random|RandomFloatinRange 0.003 0.01)) false false))

(fn ConstructionScript)