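; Custom game mode Blueprint that runs an elapsed game timer and shows it on screen.
; On BeginPlay it creates a GameTimer_Widget and adds it to the viewport.
; While player 0 has a valid pawn, Tick accumulates delta time, formats it as zero-padded minutes:seconds and writes it to the widget's text.
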(event EventBeginPlay
  (CallFunction|InitializeHUD))

(event EventTick
  (params (DeltaSeconds :type Float%20%28single-precision%29))
  (Utilities|IsValid (Game|Player|GetPlayerPawn 0)
    (:Is%20Valid
      (Variables|Default|Settime_elapsed (+ DeltaSeconds (Variables|Default|Gettime_elapsed)))
      (bind _formatted_time (CallFunction|GetFormattedGametime))
      (Utilities|IsValid (Variables|Default|Gettime_widget)
        (:Is%20Valid
          (CallFunction|UpdateUI _formatted_time))))))

(fn ConstructionScript)

(fn GetFormattedGametime
  (bind _time_elapsed (Variables|Default|Gettime_elapsed))
  (bind _returnvalue (Math|Float|Floor _time_elapsed))
  (return (Utilities|Text|FormatText "{Minutes}:{Seconds}" (Utilities|Text|ToText(Integer) (/ _returnvalue 60) false true 2 5) (Utilities|Text|ToText(Integer) (Math|Integer|%(Integer) _returnvalue 60) false false 2 5))))

(fn InitializeHUD
  (bind _returnvalue (UserInterface|CreateWidget "/Game/GUI/GameTimer_Widget.GameTimer_Widget_C"))
  (bind _output_get (Variables|Default|Settime_widget _returnvalue))
  (UserInterface|Viewport|AddtoViewport _output_get 0))

(fn UpdateUI
  (params (game_time :type Text))
  (bind _time_widget (Variables|Default|Gettime_widget))
  (Utilities|IsValid _time_widget
    (:Is%20Valid
      (Rendering|Components|TextRender|SetText (Variables|/Game/GUI/GameTimer_Widget.GameTimer_Widget_C|Getgame_time_text _time_widget) game_time))))